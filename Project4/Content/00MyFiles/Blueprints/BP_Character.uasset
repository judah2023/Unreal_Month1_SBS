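; BP_Character is a character Blueprint with health, an overhead-style HP bar widget and death handling, plus an empty Attack event.
; BeginPlay creates a WBP_HPBar for the HPBar component, caches its progress bar and fills it.
; AnyDamage subtracts clamped HP, updates the bar and calls OnDeath at zero, which sets IsDeath and disables capsule collision.
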(event `Attack`)

(event `self.ReceiveBeginPlay`
  (`|ExecutionSequence`
    (:`then_0`
      ;[1 1 1] Initialize HPBar Component
      (bind _returnvalue (`|CreateWidget` "/Game/00MyFiles/UI/WBP_HPBar.WBP_HPBar_C"))
      (`WidgetComponent.SetWidget` (`self.HP Bar`) _returnvalue))
    (:`then_1`
      ;[1 1 1] Initialize HP Bar
      (bind _aswbp_hpbar (cast `/Game/00MyFiles/UI/WBP_HPBar` (`WidgetComponent.GetUserWidgetObject` (`self.HP Bar`))))
      (bind _output_get (set `self.Progress Bar HP` (`/Game/00MyFiles/UI/WBP_HPBar.ProgressBarHP` _aswbp_hpbar)))
      (`ProgressBar.SetPercent` _output_get 1.0))))

(event `self.ReceiveAnyDamage`
  (params (Damage :type "Float (single-precision)") (DamageType :type "DamageType Object Reference") (InstigatedBy :type "Controller Object Reference") (DamageCauser :type "Actor Object Reference"))
  (`|ExecutionSequence`
    (:`then_0`
      ;[1 1 1] Decrease HP
      (set `self.HP` (`KismetMathLibrary.FClamp` (- (`self.HP`) Damage) 0.0 (`self.MaxHP`))))
    (:`then_1`
      ;[1 1 1] Update HP Bar
      (`ProgressBar.SetPercent` (`self.Progress Bar HP`) (/ (`self.HP`) (`self.MaxHP`))))
    (:`then_2`
      ;[1 1 1] Death Event
      (if (<= (`self.HP`) 0.0)
        (`self.OnDeath`)))))

(fn `OnDeath`
  (set `self.IsDeath` true)
  (`PrimitiveComponent.SetCollisionEnabled` (`self.CapsuleComponent`) "NoCollision"))

(fn `UserConstructionScript`)