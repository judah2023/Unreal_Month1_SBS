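; BP_Enemy is an enemy that wanders the navmesh at random and reports damage it receives.
; From BeginPlay, MoveEnemy picks a random reachable point within RandomRadius of its current location and moves there with AIMoveTo.
; On success or failure it waits a random delay and calls MoveEnemy again, forming an endless roam loop.
; AnyDamage only prints the damage amount, with no health or death handling.
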(event `self.ReceiveBeginPlay`
  (`self.MoveEnemy`))

(event `self.ReceiveAnyDamage`
  (params (Damage :type "Float (single-precision)") (DamageType :type "DamageType Object Reference") (InstigatedBy :type "Controller Object Reference") (DamageCauser :type "Actor Object Reference"))
  (`KismetSystemLibrary.PrintText` (`|FormatText` "Damage Hit : {Damage}" Damage)))

(event `MoveEnemy`
  (bind _output_get (set `self.Random Location` (`NavigationSystemV1.K2_GetRandomReachablePointInRadius` (`self.K2_GetActorLocation`) (`self.Random Radius`) null null)))
  (`|AIMoveTo` self _output_get null
    (:`OnSuccess`
      _)
    (:`OnFail`
      _))
  (`KismetSystemLibrary.Delay` (`KismetMathLibrary.RandomFloatInRange` 1.0 5.0))
  (`self.MoveEnemy`))

(fn `UserConstructionScript`)